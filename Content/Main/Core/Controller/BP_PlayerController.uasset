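; Player controller for the battle game that holds match state and puts the HUD and end-game screen on screen.
; On BeginPlay it binds to CPP_BattleGameMode's game-start and team-score events, storing game time and both team scores, and shows WB_HUD after a short delay.
; DisplayEndGameScreen stores the winner flag and shows WB_EndGame.
; Both screens go through a Client_ShowWidget event that creates the given widget class and adds it to the viewport.
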(event Custom|Client_ShowWidget
  (params (Class :type User%20Widget%20Class%20Reference))
  (bind _returnvalue (UserInterface|CreateWidget Class))
  (UserInterface|Viewport|AddtoViewport _returnvalue 0))

(event Custom|OnGameStarted_Event
  (params (GameTime :type Integer))
  (Variables|Default|SetGame%20Time GameTime))

(event Custom|OnTeamsScoreUpdated_Event
  (params (BlueTeamScore :type Integer) (RedTeamScore :type Integer))
  (Variables|Default|SetBlue%20Team%20Score BlueTeamScore)
  (Variables|Default|SetRed%20Team%20Score RedTeamScore))

(event EventBeginPlay
  (Utilities|FlowControl|Sequence
    (:then_0
      (bind _ascpp_battle_game_mode (Utilities|Casting|CastToCPP_BattleGameMode (Game|GetGameMode)))
      (EventDispatchers|AssignOnGameStarted _ascpp_battle_game_mode (delegate Custom|OnGameStarted_Event))
      (EventDispatchers|AssignOnTeamsScoreUpdated _ascpp_battle_game_mode (delegate Custom|OnTeamsScoreUpdated_Event)))
    (:then_1
      (Utilities|FlowControl|Delay 0.2)
      (CallFunction|ClientShowWidget "/Game/Main/UI/HUD/WB_HUD.WB_HUD_C"))))

(event EventDisplayEndGameScreen
  (params (bIsWinner :type Boolean))
  (Variables|Default|SetIs%20Winner bIsWinner)
  (CallFunction|ClientShowWidget "/Game/Main/UI/EndGameScreen/WB_EndGame.WB_EndGame_C"))

(fn ConstructionScript)