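; BP_BaseGate is a gate actor that opens when a battle starts and closes when it ends.
; On BeginPlay it binds to the battle start and end delegates of CPP_BattleGameMode, which drive MC_ControlGate, by its prefix likely a multicast event.
; Opening hides the Cube and its children and disables collision.
; Closing unhides only the Cube, not its children, and applies a blocking collision profile.
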(event Custom|OnBattleStarted_Event
  (CallFunction|MCControlGate true))

(event Custom|OnBattleEnded_Event
  (CallFunction|MCControlGate false))

(event Custom|MC_ControlGate
  (params (bOpen :type Boolean))
  (if bOpen
    (CallFunction|OpenGate)
    (else
      (CallFunction|CloseGate))))

(event EventBeginPlay
  (bind _ascpp_battle_game_mode (Utilities|Casting|CastToCPP_BattleGameMode (Game|GetGameMode)))
  (EventDispatchers|AssignOnBattleStarted _ascpp_battle_game_mode (delegate Custom|OnBattleStarted_Event))
  (EventDispatchers|AssignOnBattleEnded _ascpp_battle_game_mode (delegate Custom|OnBattleEnded_Event)))

(fn ConstructionScript)

(fn OpenGate
  (Collision|SetCollisionEnabled (Variables|Default|GetCube) "NoCollision")
  (Development|SetHiddeninGame (Variables|Default|GetCube) true true))

(fn CloseGate
  (Collision|SetCollisionEnabled (Variables|Default|GetCube) "PhysicsOnly")
  (Development|SetHiddeninGame (Variables|Default|GetCube) false false)
  (Collision|SetCollisionProfileName (Variables|Default|GetCube) "BlockAll" true :!class /Script/Engine.PrimitiveComponent))