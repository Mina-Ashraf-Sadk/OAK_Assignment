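; BP_MasterWeapon is the master weapon Blueprint, a base class for weapons held by a Character.
; On BeginPlay it caches the owning Character and its mesh AnimInstance, then seeds Ammo and Mag from WeaponDATA.
; Start and stop functions for shooting, aiming, reloading and a special action are empty here.
; UpdateAmmo overwrites the stored Ammo and Mag counts.
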(event EventBeginPlay
  (bind _ascharacter (Utilities|Casting|CastToCharacter (Components|GetOwner)))
  (bind _output_get (Variables|Default|SetCharacter _ascharacter))
  (Variables|Default|SetAnimInstance (Components|SkeletalMesh|GetAnimInstance (Variables|/Script/Engine.Character|GetMesh _output_get)))
  (Variables|Default|SetAmmo (Variables|/Game/VeilstormTasks/Data/DABP_WeaponInfo.DABP_WeaponInfo_C|GetIntialAmmo (Variables|Default|GetWeaponDATA)))
  (Variables|Default|SetMag (Variables|/Game/VeilstormTasks/Data/DABP_WeaponInfo.DABP_WeaponInfo_C|GetMagCapacity (Variables|Default|GetWeaponDATA))))

(fn ConstructionScript)

(fn StartShooting)

(fn StartAim)

(fn StartReload)

(fn StartSpeicalAction)

(fn StopShooting)

(fn StopAim)

(fn StopReload)

(fn StopSpeicalAction)

(fn UpdateAmmo
  (params (Ammo :type Integer) (Mag :type Integer))
  (Variables|Default|SetAmmo Ammo)
  (Variables|Default|SetMag Mag))